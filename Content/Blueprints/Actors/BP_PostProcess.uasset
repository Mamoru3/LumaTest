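; Post-process actor that color-grades the scene with one of three looks: Green, Warm or Blue Tone.
; Each SceneStyle value rebuilds the PostProcess component's settings with its own temperature, contrast and tint or saturation, keeping the shared post-process materials.
; The construction script applies the selected look, and Tick reapplies it every frame with the same duplicated switch.
; Pressing Q cycles SceneStyle through the three looks at runtime.
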(event EventTick
  (params (DeltaSeconds :type Float%20%28single-precision%29))
  (bind _returnvalue (Math|Float|MakeLiteralFloat 1.3))
  (bind _returnvalue_2 (Math|Float|MakeLiteralFloat 0.7))
  (bind _returnvalue_3 (Math|Float|MakeLiteralFloat 1.2))
  (bind _returnvalue_4 (Math|Float|MakeLiteralFloat 1.4))
  (switch Utilities|FlowControl|Switch|SwitchonEN_SceneStyle (Variables|Default|GetsceneStyle)
    (:NewEnumerator0
      (Variables|/Script/Engine.PostProcessComponent|SetSettings (Variables|Default|GetPostProcess) (Utilities|Struct|MakePostProcessSettings "TEMP_WhiteBalance" 4e+03 0.3 "(X=1.000000,Y=1.000000,Z=1.000000,W=1.000000)" (Math|Vector4|MakeVector4 _returnvalue_3 _returnvalue_3 _returnvalue_3 _returnvalue_3) "(X=1.000000,Y=1.000000,Z=1.000000,W=1.000000)" "(X=1.000000,Y=1.000000,Z=1.000000,W=1.000000)" "(X=1.000000,Y=1.000000,Z=1.000000,W=1.000000)" "(X=1.000000,Y=1.000000,Z=1.000000,W=1.000000)" (Variables|Default|GetPost%20Process%20Materials))))
    (:NewEnumerator1
      (Variables|/Script/Engine.PostProcessComponent|SetSettings (Variables|Default|GetPostProcess) (Utilities|Struct|MakePostProcessSettings "TEMP_WhiteBalance" 9e+03 0.2 "(X=1.000000,Y=1.000000,Z=1.000000,W=1.000000)" (Math|Vector4|MakeVector4 _returnvalue _returnvalue _returnvalue _returnvalue) "(X=1.000000,Y=1.000000,Z=1.000000,W=1.000000)" "(X=1.000000,Y=1.000000,Z=1.000000,W=1.000000)" "(X=1.000000,Y=1.000000,Z=1.000000,W=1.000000)" "(X=1.000000,Y=1.000000,Z=1.000000,W=1.000000)" (Variables|Default|GetPost%20Process%20Materials))))
    (:NewEnumerator2
      (Variables|/Script/Engine.PostProcessComponent|SetSettings (Variables|Default|GetPostProcess) (Utilities|Struct|MakePostProcessSettings "TEMP_WhiteBalance" 2.5e+03 0.0 (Math|Vector4|MakeVector4 _returnvalue_2 _returnvalue_2 _returnvalue_2 _returnvalue_2) "(X=1.000000,Y=1.000000,Z=1.000000,W=1.000000)" "(X=1.000000,Y=1.000000,Z=1.000000,W=1.000000)" "(X=1.000000,Y=1.000000,Z=1.000000,W=1.000000)" (Math|Vector4|MakeVector4 _returnvalue_4 _returnvalue_4 _returnvalue_4 _returnvalue_4) "(X=1.000000,Y=1.000000,Z=1.000000,W=1.000000)" (Variables|Default|GetPost%20Process%20Materials))))))

(event Input|KeyboardEvents|Q
  (params (Key :type Key%20Structure))
  (:Pressed
    (Variables|Default|SetsceneStyle (Utilities|Enum|ByteToEnumEN_SceneStyle (Class|KismetMathLibrary|PercentByteByte (+ (Variables|Default|GetsceneStyle) 1) 3)))))

(fn ConstructionScript
  (bind _returnvalue (Math|Float|MakeLiteralFloat 0.7))
  (bind _returnvalue_2 (Math|Float|MakeLiteralFloat 1.3))
  (bind _returnvalue_3 (Math|Float|MakeLiteralFloat 1.4))
  (switch Utilities|FlowControl|Switch|SwitchonEN_SceneStyle (Variables|Default|GetsceneStyle)
    (:NewEnumerator0
      (Variables|/Script/Engine.PostProcessComponent|SetSettings (Variables|Default|GetPostProcess) (Utilities|Struct|MakePostProcessSettings "TEMP_WhiteBalance" 4e+03 0.3 "(X=1.000000,Y=1.000000,Z=1.000000,W=1.000000)" (Math|Vector4|MakeVector4 1.2 1.2 1.2 1.2) "(X=1.000000,Y=1.000000,Z=1.000000,W=1.000000)" "(X=1.000000,Y=1.000000,Z=1.000000,W=1.000000)" "(X=1.000000,Y=1.000000,Z=1.000000,W=1.000000)" "(X=1.000000,Y=1.000000,Z=1.000000,W=1.000000)" (Variables|Default|GetPost%20Process%20Materials))))
    (:NewEnumerator1
      (Variables|/Script/Engine.PostProcessComponent|SetSettings (Variables|Default|GetPostProcess) (Utilities|Struct|MakePostProcessSettings "TEMP_WhiteBalance" 9e+03 0.2 "(X=1.000000,Y=1.000000,Z=1.000000,W=1.000000)" (Math|Vector4|MakeVector4 _returnvalue_2 _returnvalue_2 _returnvalue_2 _returnvalue_2) "(X=1.000000,Y=1.000000,Z=1.000000,W=1.000000)" "(X=1.000000,Y=1.000000,Z=1.000000,W=1.000000)" "(X=1.000000,Y=1.000000,Z=1.000000,W=1.000000)" "(X=1.000000,Y=1.000000,Z=1.000000,W=1.000000)" (Variables|Default|GetPost%20Process%20Materials))))
    (:NewEnumerator2
      (Variables|/Script/Engine.PostProcessComponent|SetSettings (Variables|Default|GetPostProcess) (Utilities|Struct|MakePostProcessSettings "TEMP_WhiteBalance" 2.5e+03 0.0 (Math|Vector4|MakeVector4 _returnvalue _returnvalue _returnvalue _returnvalue) "(X=1.000000,Y=1.000000,Z=1.000000,W=1.000000)" "(X=1.000000,Y=1.000000,Z=1.000000,W=1.000000)" "(X=1.000000,Y=1.000000,Z=1.000000,W=1.000000)" (Math|Vector4|MakeVector4 _returnvalue_3 _returnvalue_3 _returnvalue_3 _returnvalue_3) "(X=1.000000,Y=1.000000,Z=1.000000,W=1.000000)" (Variables|Default|GetPost%20Process%20Materials))))))