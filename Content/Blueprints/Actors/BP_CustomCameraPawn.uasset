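; Camera pawn with three modes, Rotating, Transitioning and VR Movement, that becomes the player's view target on BeginPlay.
; It adds a camera component matching CameraType, then forwards Enhanced Input VR controller, mouse and keyboard events to it.
; X or Backspace destroys that component to switch between Rotating and VR Movement, resetting camera transforms and HMD lock.
; In Transitioning mode, A or Enter plays a DoOnce-guarded timeline driving the component's transition.
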(event Input|EnhancedActionEvents|EnhancedInputActionMouse_RightButtonDown
  (params (ActionValue :type Boolean) (ElapsedSeconds :type Float%20%28double-precision%29) (TriggeredSeconds :type Float%20%28double-precision%29) (InputAction :type Input%20Action%20Object%20Reference :default "/Game/Input/Mouse_RightButtonDown.Mouse_RightButtonDown"))
  (bind _currentcameracomponent (Variables|Default|GetCurrentCameraComponent))
  ;[0.1166 1 0.2529] Interface Events
  (:Triggered
    (if (Utilities|Enum|Equal(Enum) (Variables|Default|GetCameraType) "NewEnumerator0") :!label _label
      (Default|RightMouseDown _currentcameracomponent ActionValue)))
  (:Started
    (goto _label))
  (:Ongoing
    (goto _label))
  (:Completed
    (Class|ICamera|RightMouseUp(Message) _currentcameracomponent)))

(event Input|EnhancedActionEvents|EnhancedInputActionRightController_AButton
  (params (ActionValue :type Boolean) (ElapsedSeconds :type Float%20%28double-precision%29) (TriggeredSeconds :type Float%20%28double-precision%29) (InputAction :type Input%20Action%20Object%20Reference :default "/Game/Input/RightController_AButton.RightController_AButton"))
  (bind _currentcameracomponent (Variables|Default|GetCurrentCameraComponent))
  (:Started
    ;[1 0.1554 0.1919] If enter is pressed and camera type is transitioning, call transition events
    (if (Utilities|Enum|Equal(Enum) (Variables|Default|GetCameraType) "NewEnumerator1")
      (Utilities|FlowControl|DoOnce false :!label _label
        (:Completed
          (bind _cameralerptime (Timeline|CameraTimeline PlayFromStart)
            (:Update
              (Default|OnUse _currentcameracomponent _cameralerptime))
            (:Finished
              (Default|OnEndUse _currentcameracomponent)
              (goto _label Reset))))))))

(event Input|EnhancedActionEvents|EnhancedInputActionRightController_BButton
  (params (ActionValue :type Boolean) (ElapsedSeconds :type Float%20%28double-precision%29) (TriggeredSeconds :type Float%20%28double-precision%29) (InputAction :type Input%20Action%20Object%20Reference :default "/Game/Input/RightController_BButton.RightController_BButton"))
  ;[0.1166 1 0.2529] Interface Events
  (:Started
    (if (Utilities|Enum|Equal(Enum) (Variables|Default|GetCameraType) "NewEnumerator0")
      (Default|OnToggle (Variables|Default|GetCurrentCameraComponent)))))

(event Input|EnhancedActionEvents|EnhancedInputActionRightControllerThumbstick_Y
  (params (ActionValue :type Float%20%28double-precision%29) (ElapsedSeconds :type Float%20%28double-precision%29) (TriggeredSeconds :type Float%20%28double-precision%29) (InputAction :type Input%20Action%20Object%20Reference :default "/Game/Input/RightControllerThumbstick_Y.RightControllerThumbstick_Y"))
  (bind _currentcameracomponent (Variables|Default|GetCurrentCameraComponent))
  (:Triggered
    (Utilities|IsValid _currentcameracomponent :!label _label
      (:Is%20Valid
        (Default|OnRightThumbstickY _currentcameracomponent ActionValue))))
  (:Started
    (goto _label))
  (:Ongoing
    (goto _label)))

(event Input|EnhancedActionEvents|EnhancedInputActionLeftControllerThumbStick_X
  (params (ActionValue :type Float%20%28double-precision%29) (ElapsedSeconds :type Float%20%28double-precision%29) (TriggeredSeconds :type Float%20%28double-precision%29) (InputAction :type Input%20Action%20Object%20Reference :default "/Game/Input/LeftControllerThumbStick_X.LeftControllerThumbStick_X"))
  (bind _currentcameracomponent (Variables|Default|GetCurrentCameraComponent))
  ;[1 0.9155 0] Rotating camera with Thumbstick
  (:Triggered
    (Utilities|IsValid _currentcameracomponent :!label _label
      (:Is%20Valid
        (Default|OnLeftThumbstickX _currentcameracomponent ActionValue))))
  (:Started
    (goto _label))
  (:Ongoing
    (goto _label)))

(event Input|EnhancedActionEvents|EnhancedInputActionLeftControllerThumbStick_Y
  (params (ActionValue :type Float%20%28double-precision%29) (ElapsedSeconds :type Float%20%28double-precision%29) (TriggeredSeconds :type Float%20%28double-precision%29) (InputAction :type Input%20Action%20Object%20Reference :default "/Game/Input/LeftControllerThumbStick_Y.LeftControllerThumbStick_Y"))
  (bind _currentcameracomponent (Variables|Default|GetCurrentCameraComponent))
  ;[1 0.9155 0] Rotating camera with Thumbstick
  (:Triggered
    (Utilities|IsValid _currentcameracomponent :!label _label
      (:Is%20Valid
        (Default|OnLeftThumbstickY _currentcameracomponent ActionValue))))
  (:Started
    (goto _label))
  (:Ongoing
    (goto _label)))

(event Input|EnhancedActionEvents|EnhancedInputActionLeftController_XButton
  (params (ActionValue :type Boolean) (ElapsedSeconds :type Float%20%28double-precision%29) (TriggeredSeconds :type Float%20%28double-precision%29) (InputAction :type Input%20Action%20Object%20Reference :default "/Game/Input/LeftController_XButton.LeftController_XButton"))
  ;[0.08632 1 0.2913] Switch between rotating camera and VRWalkingCamera
  (:Started
    (if (Utilities|Enum|Equal(Enum) (Variables|Default|GetCameraType) "NewEnumerator0")
      (Variables|Default|SetCameraType "NewEnumerator2")
      (Components|DestroyComponent (Variables|Default|GetCurrentCameraComponent))
      (bind _returnvalue (AddComponent|AddCVRMovementComponent))
      (Variables|Default|SetCurrentCameraComponent _returnvalue)
      (CallFunction|ResetVRMovementCameraPosition)
      (else
        (Variables|Default|SetCameraType "NewEnumerator0")
        (Components|DestroyComponent (Variables|Default|GetCurrentCameraComponent))
        (bind _returnvalue_2 (AddComponent|AddCRotatingCamera))
        (Variables|Default|SetCurrentCameraComponent _returnvalue_2)
        (CallFunction|ResetRotatingCameraTransform)))))

(event EventBeginPlay
  (bind _self self)
  (bind _asplayer_controller (Utilities|Casting|CastToPlayerController (Pawn|GetController)))
  (Input|AddMappingContext (PlayerController|LocalPlayerSubsystems|GetEnhancedInputLocalPlayerSubsystem _asplayer_controller) "/Game/Input/VR_InputMapping.VR_InputMapping" 0 "(bIgnoreAllPressedKeysUntilRelease=True,bForceImmediately=False)")
  (Game|Player|SetViewTargetwithBlend (Game|GetPlayerController 0) self 0.0 "VTBlend_Linear" 0.0 false)
  (switch Utilities|FlowControl|Switch|SwitchonEN_CameraType (Variables|Default|GetCameraType)
    (:NewEnumerator0
      (bind _returnvalue (AddComponent|AddCRotatingCamera _self))
      (Variables|Default|SetCurrentCameraComponent _returnvalue)
      (CallFunction|ResetRotatingCameraTransform))
    (:NewEnumerator1
      (bind _returnvalue_2 (AddComponent|AddCTransitionCamera _self))
      (Variables|Default|SetCurrentCameraComponent _returnvalue_2))
    (:NewEnumerator2
      (bind _returnvalue_3 (AddComponent|AddCVRMovementComponent))
      (Variables|Default|SetCurrentCameraComponent _returnvalue_3)
      (CallFunction|ResetVRMovementCameraPosition))))

(event Input|KeyboardEvents|SpaceBar
  (params (Key :type Key%20Structure :default "None"))
  ;[0.1166 1 0.2529] Interface Events
  (:Pressed
    (if (Utilities|Enum|Equal(Enum) (Variables|Default|GetCameraType) "NewEnumerator0")
      (Default|OnToggle (Variables|Default|GetCurrentCameraComponent)))))

(event Input|KeyboardEvents|Enter
  (params (Key :type Key%20Structure :default "None"))
  (bind _currentcameracomponent (Variables|Default|GetCurrentCameraComponent))
  (:Pressed
    ;[1 0.1554 0.1919] If enter is pressed and camera type is transitioning, call transition events
    (if (Utilities|Enum|Equal(Enum) (Variables|Default|GetCameraType) "NewEnumerator1")
      (Utilities|FlowControl|DoOnce false :!label _label
        (:Completed
          (bind _cameralerptime (Timeline|CameraTimeline PlayFromStart)
            (:Update
              (Default|OnUse _currentcameracomponent _cameralerptime))
            (:Finished
              (Default|OnEndUse _currentcameracomponent)
              (goto _label Reset))))))))

(event Input|KeyboardEvents|Backspace
  (params (Key :type Key%20Structure :default "None"))
  ;[0.08632 1 0.2913] Switch between rotating camera and VRWalkingCamera
  (:Pressed
    (if (Utilities|Enum|Equal(Enum) (Variables|Default|GetCameraType) "NewEnumerator0")
      (Variables|Default|SetCameraType "NewEnumerator2")
      (Components|DestroyComponent (Variables|Default|GetCurrentCameraComponent))
      (bind _returnvalue (AddComponent|AddCVRMovementComponent))
      (Variables|Default|SetCurrentCameraComponent _returnvalue)
      (CallFunction|ResetVRMovementCameraPosition)
      (else
        (Variables|Default|SetCameraType "NewEnumerator0")
        (Components|DestroyComponent (Variables|Default|GetCurrentCameraComponent))
        (bind _returnvalue_2 (AddComponent|AddCRotatingCamera))
        (Variables|Default|SetCurrentCameraComponent _returnvalue_2)
        (CallFunction|ResetRotatingCameraTransform)))))

(fn ConstructionScript
  (switch Utilities|FlowControl|Switch|SwitchonEN_CameraType (Variables|Default|GetCameraType)
    (:NewEnumerator0
      (Variables|/Script/Engine.CameraComponent|SetbLockToHmd (Variables|Default|GetCamera) false :!label _label))
    (:NewEnumerator1
      (goto _label))
    (:NewEnumerator2
      (Variables|/Script/Engine.CameraComponent|SetbLockToHmd (Variables|Default|GetCamera) true))
    (:NewEnumerator3
      (goto _label))))

(fn ResetVRMovementCameraPosition
  (bind _camerascenecomponent (Variables|Default|GetCameraSceneComponent))
  (bind _camera (Variables|Default|GetCamera))
  (Transformation|SetWorldScale3D _camera "1.000000,1.000000,1.000000")
  (Transformation|SetWorldRotation _camera "0, 0, 0" false false)
  (Transformation|SetWorldLocation _camerascenecomponent "300.000000,-105.000000,300.000000" false false)
  (Transformation|SetRelativeRotation _camerascenecomponent "0, 0, 0" false false)
  (Variables|/Script/Engine.CameraComponent|SetbLockToHmd (Variables|Default|GetCamera) true))

(fn ResetRotatingCameraTransform
  (Transformation|SetRelativeTransform (Variables|Default|GetCamera) (Math|Transform|MakeTransform (Math|Vector|MakeVector -268.0 0.0 248.0) (Math|Rotator|MakeRotator 0.0 -5e+01 0.0)) false false)
  (Transformation|SetWorldLocation (Variables|Default|GetCameraSceneComponent) "755.000000,-123.000000,462.679171" false false)
  (Variables|/Script/Engine.CameraComponent|SetbLockToHmd (Variables|Default|GetCamera) false))