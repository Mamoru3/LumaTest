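; Camera actor that becomes the player's view target on BeginPlay and runs as either a rotating or transitioning camera.
; CameraType selects which component to add in both the construction script and BeginPlay; Rotating also repositions the Camera.
; Right mouse and Space inputs are forwarded to the current component through interface calls.
; In Transitioning mode, Enter plays a DoOnce-guarded timeline that feeds lerp time to the component, then signals completion.
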(event EventBeginPlay
  (bind _self self)
  (Game|Player|SetViewTargetwithBlend (Game|GetPlayerController 0) self 0.0 "VTBlend_Linear" 0.0 false)
  (switch Utilities|FlowControl|Switch|SwitchonEN_CameraType (Variables|Default|GetCameraType)
    (:NewEnumerator0
      (bind _returnvalue (AddComponent|AddCRotatingCamera _self))
      (Transformation|SetRelativeTransform (Variables|Default|GetCamera) (Math|Transform|MakeTransform (Math|Vector|MakeVector -67.0 0.0 62.0) (Math|Rotator|MakeRotator 0.0 -5e+01 0.0)) false false)
      (Variables|Default|SetCurrentCameraComponent _returnvalue))
    (:NewEnumerator1
      (bind _returnvalue_2 (AddComponent|AddCTransitionCamera _self))
      (Variables|Default|SetCurrentCameraComponent _returnvalue_2))))

(event Input|KeyboardEvents|SpaceBar
  (params (Key :type Key%20Structure :default "None"))
  ;[0.1166 1 0.2529] Interface Events
  (:Pressed
    (Default|OnToggle (Variables|Default|GetCurrentCameraComponent))))

(event Input|KeyboardEvents|Enter
  (params (Key :type Key%20Structure :default "None"))
  (bind _currentcameracomponent (Variables|Default|GetCurrentCameraComponent))
  (:Pressed
    (if (Utilities|Enum|Equal(Enum) (Variables|Default|GetCameraType) "NewEnumerator1")
      ;[1 0.1554 0.1919] If enter is pressed and camera type is transitioning, call transition events
      (Utilities|FlowControl|DoOnce false :!label _label
        (:Completed
          (bind _cameralerptime (Timeline|CameraTimeline PlayFromStart)
            (:Update
              (Default|OnUse _currentcameracomponent _cameralerptime))
            (:Finished
              (Default|OnEndUse _currentcameracomponent)
              (goto _label Reset))))))))

(event Input|MouseEvents|RightMouseButton
  (params (Key :type Key%20Structure :default "None"))
  (bind _currentcameracomponent (Variables|Default|GetCurrentCameraComponent))
  ;[0.1166 1 0.2529] Interface Events
  (:Pressed
    (Default|RightMouseDown _currentcameracomponent true))
  (:Released
    (Default|RightMouseDown _currentcameracomponent false)))

(fn ConstructionScript
  (switch Utilities|FlowControl|Switch|SwitchonEN_CameraType (Variables|Default|GetCameraType)
    (:NewEnumerator0
      (bind _returnvalue (AddComponent|AddCRotatingCamera))
      (Transformation|SetRelativeTransform (Variables|Default|GetCamera) (Math|Transform|MakeTransform (Math|Vector|MakeVector -67.0 0.0 62.0) (Math|Rotator|MakeRotator 0.0 -5e+01 0.0)) false false)
      (Variables|Default|SetCurrentCameraComponent _returnvalue))
    (:NewEnumerator1
      (bind _returnvalue_2 (AddComponent|AddCTransitionCamera))
      (Variables|Default|SetCurrentCameraComponent _returnvalue_2))))