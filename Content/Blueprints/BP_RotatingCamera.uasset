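; A camera actor that becomes the player's view target on BeginPlay and rotates its Scene component, either automatically or by mouse drag.
; Space toggles between a constant yaw spin scaled by RotationSpeed and delta time, and mouse rotation.
; In mouse mode, Tick tracks the viewport cursor and, while the right button is held, feeds movement deltas above a small threshold into RotateSceneRoot, which clamps pitch.
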(event EventBeginPlay
  (Game|Player|SetViewTargetwithBlend (Game|GetPlayerController 0) self 0.0 "VTBlend_Linear" 0.0 false)
  (bind _returnvalue (Class|WidgetLayoutLibrary|GetMousePositiononViewport))
  (bind _output_get (Variables|Default|SetoldMousePos _returnvalue))
  (Variables|Default|SetcurrentPos _output_get))

(event EventTick
  (params (DeltaSeconds :type Float%20%28single-precision%29))
  (Utilities|FlowControl|Sequence
    (:then_0
      (if (Variables|Default|GetuseMouseRotation)
        (if (Variables|Default|GetIsRightMouseDown)
          (bind _returnvalue (Class|WidgetLayoutLibrary|GetMousePositiononViewport))
          (Variables|Default|SetcurrentPos _returnvalue)
          (if (> (Math|Vector2D|Vector2DLength (- (Variables|Default|GetcurrentPos) (Variables|Default|GetoldMousePos))) 0.8)
            (CallFunction|RotateSceneRoot (- (Variables|Default|GetcurrentPos) (Variables|Default|GetoldMousePos)))
            (Variables|Default|SetoldMousePos (Variables|Default|GetcurrentPos)))
          (else
            (bind _returnvalue_2 (Class|WidgetLayoutLibrary|GetMousePositiononViewport))
            (Variables|Default|SetcurrentPos _returnvalue_2)))
        (else
          (CallFunction|ConstantCameraRotation))))))

(event Input|MouseEvents|RightMouseButton
  (params (Key :type Key%20Structure :default "None"))
  (:Pressed
    (Variables|Default|SetIsRightMouseDown true)
    (Variables|Default|SetoldMousePos (Variables|Default|GetcurrentPos)))
  (:Released
    (Variables|Default|SetIsRightMouseDown false)))

(event Input|KeyboardEvents|SpaceBar
  (params (Key :type Key%20Structure :default "None"))
  (:Pressed
    (Variables|Default|SetuseMouseRotation (not (Variables|Default|GetuseMouseRotation)))))

(fn ConstructionScript)

(fn ConstantCameraRotation
  (bind _scene (Variables|Default|GetScene))
  (bind _relativerotation (Variables|/Script/Engine.SceneComponent|GetRelativeRotation _scene))
  (Transformation|SetRelativeRotation _scene (Math|Rotator|MakeRotator (.roll _relativerotation) (.pitch _relativerotation) (- (.yaw _relativerotation) (* (Utilities|Time|GetWorldDeltaSeconds) (Variables|Default|GetrotationSpeed)))) false false))

(fn RotateSceneRoot
  (params (RotationVector :type Vector%202D%20Structure))
  (bind _scene (Variables|Default|GetScene))
  (bind _relativerotation (Variables|/Script/Engine.SceneComponent|GetRelativeRotation _scene))
  ;[1 0.6577 0.3139] Rotate using mouse
  (Transformation|SetRelativeRotation _scene (Math|Rotator|MakeRotator (.roll _relativerotation) (Math|Float|Clamp(Float) (+ (.pitch _relativerotation) (.Y (Math|Vector2D|BreakVector2D RotationVector))) -11.0 53.0) (+ (.yaw _relativerotation) (.X (Math|Vector2D|BreakVector2D RotationVector)))) false false))