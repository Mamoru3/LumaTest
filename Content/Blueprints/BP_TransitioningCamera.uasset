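; BP_TransitioningCamera is a key-driven camera switcher that hands the transition work to its CTransitionCamera component.
; Space Bar requests the next cycled camera, then either blends to it by feeding a timeline value into LerpToNextCamera or teleports to it, depending on the component's lerp setting.
; Enter toggles that lerp setting.
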(event EventBeginPlay)

(event Collision|EventActorBeginOverlap
  (params (OtherActor :type Actor%20Object%20Reference)))

(event EventTick
  (params (DeltaSeconds :type Float%20%28single-precision%29)))

(event Input|KeyboardEvents|Enter
  (params (Key :type Key%20Structure :default "None"))
  (:Pressed
    (Default|ToggleLerptoCameras (Variables|Default|GetC_TransitionCamera))))

(event Input|KeyboardEvents|SpaceBar
  (params (Key :type Key%20Structure :default "None"))
  (bind _c_transitioncamera (Variables|Default|GetC_TransitionCamera))
  (:Pressed
    (Default|GetNextCycledCamera _c_transitioncamera)
    (if (Default|GetLerptoCamera _c_transitioncamera)
      (bind _value (Timeline|Timeline PlayFromStart)
        (:Update
          (Default|LerptoNextCamera (Variables|Default|GetC_TransitionCamera) _value)))
      (else
        (Default|TeleporttoNextCamera (Variables|Default|GetC_TransitionCamera))))))

(fn ConstructionScript
  (|CallParentFunction))