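; Camera component that orbits the parent camera's scene component, toggling between automatic spin and user control.
; When custom rotation is off, Tick applies a constant yaw and keeps the stored mouse position current.
; When on, right-mouse drag deltas or left thumbstick drive yaw and clamped pitch.
; Right thumbstick moves the camera along the line to the pivot, restoring its last position when too close.
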(event EventBeginPlay
  ;[0.2399 0.08185 1] Init
  (|CallParentFunction)
  (CallFunction|UpdateCurrentMousePos)
  (Variables|Default|SetoldMousePos (Variables|Default|GetcurrentPos)))

(event EventTick
  (params (DeltaSeconds :type Float%20%28single-precision%29))
  ;[0.1448 0.2646 1] If thumbstick is moving, use VR controller, else mouse is being used
  (Development|PrintString (Utilities|String|ToString(Boolean) (Variables|Default|GetuseCustomRotation)))
  (if (Variables|Default|GetuseCustomRotation)
    (CallFunction|UpdateCurrentMousePos)
    (else
      ;[0.8108 0.28 1] If mouse is not being used, apply constant rotation
      (CallFunction|UpdateCurrentMousePos)
      (Variables|Default|SetoldMousePos (Variables|Default|GetcurrentPos))
      (CallFunction|ConstantCameraRotation))))

(event EventOnLeftThumbstickX
  (params (LeftThumbstickX :type Float%20%28double-precision%29))
  (bind _parentcamera (Variables|Default|GetParentCamera))
  (bind _camerascenecomponent (Variables|/Game/Blueprints/Actors/BP_CustomCameraPawn.BP_CustomCameraPawn_C|GetCameraSceneComponent _parentcamera))
  (bind _relativerotation (Variables|/Script/Engine.SceneComponent|GetRelativeRotation _camerascenecomponent))
  ;[0 1 0.8418] Rotate camera left and right using left thumbstick
  (if (Variables|Default|GetuseCustomRotation)
    (Transformation|SetRelativeRotation _camerascenecomponent (Math|Rotator|MakeRotator (.roll _relativerotation) (.pitch _relativerotation) (+ (* (* LeftThumbstickX (Variables|Default|GetrotationSpeed)) -1.0) (.yaw _relativerotation))) false false)))

(event EventOnRightThumbstickY
  (params (Value :type Float%20%28double-precision%29))
  (bind _returnvalue (CallFunction|GetCameratoCameraSceneComponentVector))
  (bind _parentcamera (Variables|Default|GetParentCamera))
  (bind _parentcamera_2 (Variables|Default|GetParentCamera))
  (bind _camera (Variables|/Game/Blueprints/Actors/BP_CustomCameraPawn.BP_CustomCameraPawn_C|GetCamera _parentcamera))
  (bind _camera_2 (Variables|/Game/Blueprints/Actors/BP_CustomCameraPawn.BP_CustomCameraPawn_C|GetCamera _parentcamera_2))
  (bind _returnvalue_2 (Transformation|GetWorldLocation _camera))
  ;[0.7415 0.007103 1] Move camera towards scene component, limit when too close
  (if (Variables|Default|GetuseCustomRotation)
    (if (>= (Math|Vector|VectorLength _returnvalue) 5e+01)
      (bind _output_get (Variables|Default|SetcurrentPos3D _returnvalue_2))
      (Transformation|SetWorldLocation _camera_2 (+ _returnvalue_2 (* (Math|Vector|Normalize _returnvalue) (* Value (Variables|Default|GetMovingSpeed)))) false false)
      (Variables|Default|SetlastPos3D _output_get)
      (else
        (Transformation|SetWorldLocation _camera_2 (Variables|Default|GetlastPos3D) false false)))))

(event EventOnToggle
  ;[1 0.9823 0.03889] Interface Calls
  (Variables|Default|SetuseCustomRotation (not (Variables|Default|GetuseCustomRotation))))

(event EventRightMouseDown
  (params (IsDown :type Boolean))
  ;[1 0.9823 0.03889] Interface Calls
  (if (Variables|Default|GetuseCustomRotation)
    (CallFunction|MouseCameraRotation IsDown)))

(event EventOnLeftThumbstickY
  (params (LeftThumbstickY :type Float%20%28double-precision%29))
  (bind _parentcamera (Variables|Default|GetParentCamera))
  (bind _camerascenecomponent (Variables|/Game/Blueprints/Actors/BP_CustomCameraPawn.BP_CustomCameraPawn_C|GetCameraSceneComponent _parentcamera))
  (bind _relativerotation (Variables|/Script/Engine.SceneComponent|GetRelativeRotation _camerascenecomponent))
  ;[0.1573 1 0.2027] Rotate Camera up and down using left thumbstick
  (if (Variables|Default|GetuseCustomRotation)
    (Transformation|SetRelativeRotation _camerascenecomponent (Math|Rotator|MakeRotator (.roll _relativerotation) (Math|Float|Clamp(Float) (+ (.pitch _relativerotation) (* LeftThumbstickY (Variables|Default|GetrotationSpeed))) -11.0 53.0) (.yaw _relativerotation)) false false)))

(fn RotateSceneRoot
  (params (RotationVector :type Vector%202D%20Structure))
  (bind _parentcamera (Variables|Default|GetParentCamera))
  (bind _camerascenecomponent (Variables|/Game/Blueprints/Actors/BP_CustomCameraPawn.BP_CustomCameraPawn_C|GetCameraSceneComponent _parentcamera))
  (bind _relativerotation (Variables|/Script/Engine.SceneComponent|GetRelativeRotation _camerascenecomponent))
  ;[1 0.6577 0.3139] Rotate using mouse
  (Transformation|SetRelativeRotation _camerascenecomponent (Math|Rotator|MakeRotator (.roll _relativerotation) (Math|Float|Clamp(Float) (+ (.pitch _relativerotation) (.Y (Math|Vector2D|BreakVector2D RotationVector))) -11.0 53.0) (+ (.yaw _relativerotation) (.X (Math|Vector2D|BreakVector2D RotationVector)))) false false))

(fn UpdateCurrentMousePos
  (bind _returnvalue (Class|WidgetLayoutLibrary|GetMousePositiononViewport))
  (Variables|Default|SetcurrentPos _returnvalue))

(fn ConstantCameraRotation
  (bind _parentcamera (Variables|Default|GetParentCamera))
  (bind _camerascenecomponent (Variables|/Game/Blueprints/Actors/BP_CustomCameraPawn.BP_CustomCameraPawn_C|GetCameraSceneComponent _parentcamera))
  (bind _relativerotation (Variables|/Script/Engine.SceneComponent|GetRelativeRotation _camerascenecomponent))
  (Transformation|SetRelativeRotation _camerascenecomponent (Math|Rotator|MakeRotator (.roll _relativerotation) (.pitch _relativerotation) (- (.yaw _relativerotation) (* (Variables|Default|GetrotationSpeed) (Utilities|Time|GetWorldDeltaSeconds)))) false false))

(fn ThumbstickCameraRotation
  (bind _parentcamera (Variables|Default|GetParentCamera))
  (bind _camerascenecomponent (Variables|/Game/Blueprints/Actors/BP_CustomCameraPawn.BP_CustomCameraPawn_C|GetCameraSceneComponent _parentcamera))
  (bind _relativerotation (Variables|/Script/Engine.SceneComponent|GetRelativeRotation _camerascenecomponent))
  (Transformation|SetRelativeRotation _camerascenecomponent (Math|Rotator|MakeRotator (.roll _relativerotation) (.pitch _relativerotation) (- (.yaw _relativerotation) (* (Variables|Default|GetrotationSpeed) (Utilities|Time|GetWorldDeltaSeconds)))) false false))

(fn MouseCameraRotation
  (params (IsButtonDown :type Boolean))
  ;[0.05076 1 0.0751] Calculate mouse movement direction vector and update root rotation
  (if IsButtonDown
    (CallFunction|UpdateCurrentMousePos)
    (if (> (Math|Vector2D|Vector2DLength (- (Variables|Default|GetcurrentPos) (Variables|Default|GetoldMousePos))) 0.8)
      (CallFunction|RotateSceneRoot (- (Variables|Default|GetcurrentPos) (Variables|Default|GetoldMousePos)))
      (Variables|Default|SetoldMousePos (Variables|Default|GetcurrentPos)))
    (else
      (CallFunction|UpdateCurrentMousePos))))

(fn GetCameratoCameraSceneComponentVector
  (bind _parentcamera (Variables|Default|GetParentCamera))
  (return (- (Transformation|GetWorldLocation (Variables|/Game/Blueprints/Actors/BP_CustomCameraPawn.BP_CustomCameraPawn_C|GetCameraSceneComponent _parentcamera)) (Transformation|GetWorldLocation (Variables|/Game/Blueprints/Actors/BP_CustomCameraPawn.BP_CustomCameraPawn_C|GetCamera _parentcamera)))))