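; C_TransitionCamera is a component for BP_CustomCameraActor that moves its camera between BP_CameraTarget actors in the level.
; BeginPlay caches the owner and all targets, and GetNextCycledCamera selects the next one by wrapping index.
; Events either snap the camera's scene component to that target or lerp from its current transform, using the caller's timeline value over a divider.
; A toggleable flag, exposed through a getter, records whether lerping is wanted.
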(event Custom|LerpToNextCamera
  (params (TimelineSpeed :type Float%20%28double-precision%29))
  (bind _maincamera (Variables|Default|GetmainCamera))
  (bind _camerascenecomponent (Variables|/Game/Blueprints/BP_CustomCameraActor.BP_CustomCameraActor_C|GetCameraSceneComponent _maincamera))
  (Transformation|SetWorldTransform _camerascenecomponent (Math|Transform|Lerp(Transform) (Transformation|GetWorldTransform _camerascenecomponent) (Transformation|GetActorTransform (Variables|Default|GetNextCamera)) (/ TimelineSpeed (Variables|Default|GetLerpSpeedDivider))) false false))

(event Custom|ToggleLerpToCameras
  (Variables|Default|SetlerpToCamera (not (Variables|Default|GetlerpToCamera))))

(event Custom|TeleportToNextCamera
  (Transformation|SetWorldTransform (Variables|/Game/Blueprints/BP_CustomCameraActor.BP_CustomCameraActor_C|GetCameraSceneComponent (Variables|Default|GetmainCamera)) (Transformation|GetActorTransform (Variables|Default|GetNextCamera)) false false))

(event EventBeginPlay
  (bind _asbp_custom_camera_actor (Utilities|Casting|CastToBP_CustomCameraActor (Components|GetOwner)))
  (Variables|Default|SetmainCamera _asbp_custom_camera_actor)
  (bind _outactors (Actor|GetAllActorsOfClass "/Game/Blueprints/BP_CameraTarget.BP_CameraTarget_C"))
  (Variables|Default|SetcameraTargets _outactors))

(fn GetNextCycledCamera
  (bind _cameratargets (Variables|Default|GetcameraTargets))
  (bind _cameratargetindex (Variables|Default|GetcameraTargetIndex))
  (Math|Integer|IncrementInt _cameratargetindex
    (:%20%20
      (Variables|Default|SetNextCamera (Utilities|Array|Get(acopy) _cameratargets (Math|Integer|%(Integer) _cameratargetindex (Utilities|Array|Length _cameratargets))))
      (return))))

(fn GetLerptoCamera
  (return (Variables|Default|GetlerpToCamera)))