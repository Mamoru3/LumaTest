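; Camera manager that moves the first CameraActor found in the level between all BP_CameraTarget actors gathered on BeginPlay.
; Space Bar cycles to the next target through a wrapping index, and Enter toggles between snapping and smooth movement.
; Smooth moves use a Timeline in an EventGraph event, lerping from the camera's current transform each update by timeline value over a speed divider.
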(event Custom|LerpToNextCamera
  (params (currentCycledCamera :type BP%20Camera%20Target%20Object%20Reference))
  (bind _maincamera (Variables|Default|GetmainCamera))
  (bind _scenecomponent (Variables|/Script/Engine.CameraActor|GetSceneComponent _maincamera))
  ;[0.1211 0.0913 1] Lerp to next Cycled camera event, Timeline not available in Functions
  (bind _cameralerptime (Timeline|CameraLerp PlayFromStart)
    (:Update
      (Transformation|SetWorldTransform _scenecomponent (Math|Transform|Lerp(Transform) (Transformation|GetWorldTransform _scenecomponent) (Transformation|GetActorTransform currentCycledCamera) (/ _cameralerptime (Variables|Default|GetLerpSpeedDivider))) false false))))

(event EventBeginPlay
  ;[0.3615 0.9402 1] Get Possessed camera and get all Camera Targets
  (CallFunction|GetFirstCamera)
  (bind _outactors (Actor|GetAllActorsOfClass "/Game/Blueprints/BP_CameraTarget.BP_CameraTarget_C"))
  (Variables|Default|SetcameraTargets _outactors))

(event Input|KeyboardEvents|SpaceBar
  (params (Key :type Key%20Structure :default "None"))
  (:Pressed
    (CallFunction|CameraCycle)))

(event Input|KeyboardEvents|Enter
  (params (Key :type Key%20Structure :default "None"))
  (:Pressed
    (Variables|Default|SetlerpToCameras (not (Variables|Default|GetlerpToCameras)))))

(fn ConstructionScript)

(fn GetFirstCamera
  (bind _outactors (Actor|GetAllActorsOfClass "/Script/Engine.CameraActor"))
  (if (not (Utilities|Array|IsEmpty _outactors))
    (Variables|Default|SetmainCamera (Utilities|Array|Get(acopy) _outactors))))

(fn CameraCycle
  (bind _output (CallFunction|GetNextCycledCamera))
  (if (Variables|Default|GetlerpToCameras)
    (CallFunction|LerptoNextCamera _output)
    (else
      (Transformation|SetWorldTransform (Variables|/Script/Engine.CameraActor|GetSceneComponent (Variables|Default|GetmainCamera)) (Transformation|GetActorTransform _output) false false))))

(fn GetNextCycledCamera
  (bind _cameratargets (Variables|Default|GetcameraTargets))
  (bind _cameratargetindex (Variables|Default|GetcameraTargetIndex))
  (Math|Integer|IncrementInt _cameratargetindex
    (:%20%20
      (return (Utilities|Array|Get(acopy) _cameratargets (Math|Integer|%(Integer) _cameratargetindex (Utilities|Array|Length _cameratargets)))))))